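; A 3D pop-up panel actor, named as a button-less variant, that uses its background and text widgets as the accept control.
; On BeginPlay it binds both widgets' button-press events to OnAcceptButtonPressed, which defers to the parent implementation.
; It then enables player input, sets up widget interaction references, calls GetGameManager, and starts a fast looping timer on UpdateRotation instead of using Tick.
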(event `self.OnAcceptButtonPressed`
  (params (ClickedWidget :type "/Game/Widgets/PopUps/BaseWidget Object Reference"))
  (`parent.OnAcceptButtonPressed` null))

(event `self.ReceiveBeginPlay`
  (`|ExecutionSequence`
    (:`then_0`
      (bind _asbase_widget (cast `/Game/Widgets/PopUps/BaseWidget` (`WidgetComponent.GetUserWidgetObject` (`self.BackgroundPanel`)))
        (:`then`
          (bind _asbase_widget_2 (cast `/Game/Widgets/PopUps/BaseWidget` (`WidgetComponent.GetUserWidgetObject` (`self.Text`)))))
        (:`CastFailed`
          _))
      (add `/Game/Widgets/PopUps/BaseWidget.OnButtonPressed` _asbase_widget_2 (delegate `self.OnAcceptButtonPressed`))
      (add `/Game/Widgets/PopUps/BaseWidget.OnButtonPressed` _asbase_widget (delegate `self.OnAcceptButtonPressed`)))
    (:`then_1`
      (`self.EnableInput` (`GameplayStatics.GetPlayerController` 0))
      (`self.SetWidgetInteractionReferences`)
      (`self.GetGameManager`)
      (`KismetSystemLibrary.K2_SetTimer` null "UpdateRotation" 0.001 true))))

(fn `UserConstructionScript`
  (`parent.UserConstructionScript`))