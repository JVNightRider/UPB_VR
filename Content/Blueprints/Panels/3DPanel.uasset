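; A world-space 3D pop-up panel with text, a tinted background and accept and optional cancel buttons.
; SetupPanel configures the contents, colour, justification and size offset through widget components.
; Button presses set flags, while tapping the text reports any assigned glossary word to the GameManager's SceneFlowManager.
; A looping timer started in the construction script turns the panel mesh on yaw to face the player camera.
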(event `OnAcceptButtonPressed`
  (params (ClickedWidget :type "/Game/Widgets/PopUps/BaseWidget Object Reference"))
  ;[1 1 1] Detect Accept And Cancel Buttons pressed
  (set `self.isButton1Pressed` true))

(event `OnTextPanelPressed`
  (params (ClickedWidget :type "/Game/Widgets/PopUps/BaseWidget Object Reference"))
  ;[1 1 1] Detect glossary Text Tapped
  (if (`|EnumInequality` (`self.glossaryWord`) "NewEnumerator6")
    (`/Game/Blueprints/Managers/SceneFlowManager.GlossaryWordTaped` (`/Game/Blueprints/Managers/GameManager.SceneFlowManager` (`self.GameManager`)) (`self.glossaryWord`) self)))

(event `OnCancelButtonPressed`
  (params (ClickedWidget :type "/Game/Widgets/PopUps/BaseWidget Object Reference"))
  ;[1 1 1] Detect Accept And Cancel Buttons pressed
  (set `self.isButton2Pressed` true))

(event `self.ReceiveBeginPlay`
  (bind _asbase_widget (cast `/Game/Widgets/PopUps/BaseWidget` (`WidgetComponent.GetUserWidgetObject` (`self.Button1`)))
    (:`then`
      (add `/Game/Widgets/PopUps/BaseWidget.OnButtonPressed` _asbase_widget (delegate `OnAcceptButtonPressed`)))
    (:`CastFailed`
      _))
  (bind _asbase_widget_2 (cast `/Game/Widgets/PopUps/BaseWidget` (`WidgetComponent.GetUserWidgetObject` (`self.Button2`)))
    (:`then`
      (add `/Game/Widgets/PopUps/BaseWidget.OnButtonPressed` _asbase_widget_2 (delegate `OnCancelButtonPressed`)))
    (:`CastFailed`
      _))
  (bind _asbase_widget_3 (cast `/Game/Widgets/PopUps/BaseWidget` (`WidgetComponent.GetUserWidgetObject` (`self.Text`))))
  (add `/Game/Widgets/PopUps/BaseWidget.OnButtonPressed` _asbase_widget_3 (delegate `OnTextPanelPressed`)))

(event `GetGameManager`
  (bind _returnvalue (`GameplayStatics.GetActorOfClass` "/Game/Blueprints/Managers/GameManager.GameManager_C"))
  (`/Engine/EditorBlueprintResources/StandardMacros.IsValid` _returnvalue
    (:`Is Valid`
      (set `self.GameManager` _returnvalue))))

(event `SetupPanel`
  (params (text :type String) (b_useCancelButton :type Boolean) (pivot :type "SceneComponent Object Reference") (`Tint Color Specified Color` :type "LinearColor Structure" :default (struct :`R` 1.0 :`G` 1.0 :`B` 1.0 :`A` 1.0)) (Justification :type "ETextJustify Enum" :default "Left") (TextButton1 :type String) (TextButton2 :type String) (glossaryWord :type "/Game/Blueprints/Enums/GlossaryWords Enum" :default "NewEnumerator6") (OffsetSize :type "Vector2D Structure"))
  (bind _asbase_widget (cast `/Game/Widgets/PopUps/BaseWidget` (`WidgetComponent.GetUserWidgetObject` (`self.Text`)))
    (:`then`
      (`/Game/Widgets/PopUps/BaseWidget.SetText` _asbase_widget text))
    (:`CastFailed`
      _))
  (`SceneComponent.SetVisibility` (`self.Button2`) b_useCancelButton false)
  (`self.SetActorScale3D` (0.1 0.1 0.1))
  (`self.SetColorPanel` `Tint Color Specified Color`)
  (`self.SetJustification` Justification)
  (`self.SetButton1Text` TextButton1)
  (`self.SetButton2Text` TextButton2)
  (`self.SetOffsetSize` OffsetSize)
  (set `self.glossaryWord` glossaryWord))

(event `SetColorPanel`
  (params (`Tint Color Specified Color` :type "LinearColor Structure"))
  (bind _assimple_panel_color_widget (cast `/Game/Widgets/PopUps/SimplePanelColorWidget` (`WidgetComponent.GetUserWidgetObject` (`self.BackgroundPanel`))))
  (`/Game/Widgets/PopUps/SimplePanelColorWidget.SetPanelColor` _assimple_panel_color_widget `Tint Color Specified Color`))

(event `SetJustification`
  (params (Justification :type "ETextJustify Enum" :default "Left"))
  (bind _assimple_text_panel_widget (cast `/Game/Widgets/PopUps/SimpleTextPanelWidget` (`WidgetComponent.GetUserWidgetObject` (`self.Text`))))
  (`/Game/Widgets/PopUps/SimpleTextPanelWidget.SetJustification` _assimple_text_panel_widget Justification))

(event `SetButton1Text`
  (params (Text :type String))
  (bind _asbase_widget (cast `/Game/Widgets/PopUps/BaseWidget` (`WidgetComponent.GetUserWidgetObject` (`self.Button1`))))
  (if (!= Text "")
    (`/Game/Widgets/PopUps/BaseWidget.SetText` _asbase_widget Text)))

(event `SetButton2Text`
  (params (Text :type String))
  (bind _asbase_widget (cast `/Game/Widgets/PopUps/BaseWidget` (`WidgetComponent.GetUserWidgetObject` (`self.Button2`))))
  (if (!= Text "")
    (`/Game/Widgets/PopUps/BaseWidget.SetText` _asbase_widget Text)))

(event `SetOffsetSize`
  (params (Size :type "Vector2D Structure"))
  (bind _text (`self.Text`))
  (bind _backgroundpanel (`self.BackgroundPanel`))
  (`WidgetComponent.SetDrawSize` _text (+ Size (`WidgetComponent.GetDrawSize` _text)))
  (`WidgetComponent.SetDrawSize` _backgroundpanel (+ Size (`WidgetComponent.GetDrawSize` _backgroundpanel))))

(event `DeletePanel`
  (`self.K2_DestroyActor`))

(fn `UpdateRotation`
  (`SceneComponent.K2_SetWorldRotation` (`self.SM_ObjectPanel`) (`KismetMathLibrary.MakeRotator` 0.0 0.0 (+ (.yaw (`KismetMathLibrary.FindLookAtRotation` (`SceneComponent.K2_GetComponentLocation` (`self.SM_ObjectPanel`)) (`PlayerCameraManager.GetCameraLocation` (`PlayerController.PlayerCameraManager` (`GameplayStatics.GetPlayerController` 0))))) 90.0)) false false))

(fn `UserConstructionScript`
  (`self.GetGameManager`)
  (`KismetSystemLibrary.K2_SetTimer` null "UpdateRotation" 0.001 true))