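; 3D BeFast pop-up panel: a child panel actor with five toggle answers, a Spanish confirmation prompt and scoring.
; Setup restores and locks answers saved in the GameManager's PopUpsManager.
; Accept reveals the confirmation by scaling it up and disables toggle collision; Yes adds ScoreAnswers points for newly selected toggles before running the parent accept.
; Per-toggle confirmation binding is disconnected, and CorrectAnswers is stored but unused in scoring.
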(event `self.SetupPanel`
  (params (text :type String) (b_useCancelButton :type Boolean) (pivot :type "SceneComponent Object Reference") (`Tint Color Specified Color` :type "LinearColor Structure") (Justification :type "ETextJustify Enum" :default "Left") (TextButton1 :type String) (TextButton2 :type String) (glossaryWord :type "/Game/Blueprints/Enums/GlossaryWords Enum" :default "NewEnumerator6") (OffsetSize :type "Vector2D Structure"))
  (`parent.SetupPanel` text b_useCancelButton pivot `Tint Color Specified Color` Justification TextButton1 TextButton2 glossaryWord OffsetSize)
  (`self.SetActorScale3D` (0.132357 0.132357 0.132357))
  ;[1 1 1] Togggle On The saved answers
  (for (_array_element _array_index) (`self.Toggles`)
    (bind _assimple_toggle_box (cast `/Game/Widgets/PopUps/SimpleToggleBox` (`WidgetComponent.GetUserWidgetObject` _array_element)))
    (if (`|GetArrayItem` (`/Game/Blueprints/Managers/PopUpsManager.ToggleAnswers` (`/Game/Blueprints/Managers/GameManager.PopUpsManager` (`self.GameManager`))) _array_index)
      (`/Game/Widgets/PopUps/SimpleToggleBox.SetToggleValue` _assimple_toggle_box true)
      (set `/Game/Widgets/PopUps/SimpleToggleBox.b_LockSelection` true _assimple_toggle_box))))

(event `SetScoreAnswers`
  (params (ScoreAnswers :type "Array of Integer"))
  (set `self.ScoreAnswers` ScoreAnswers))

(event `SetRightAnswers`
  (params (CorrectAnswers :type "Array of Boolean"))
  (set `self.CorrectAnswers` CorrectAnswers))

(event `self.OnAcceptButtonPressed`
  (params (ClickedWidget :type "/Game/Widgets/PopUps/BaseWidget Object Reference"))
  ;[1 1 1] On Accept Button Pressed
  (`self.ShowConfirmationPanel`))

(event `OnTogglePressed`
  (params (ClickedWidget :type "/Game/Widgets/PopUps/BaseWidget Object Reference"))
  ;[1 1 1] Detect when a toggle change value
  (bind _assimple_toggle_box (cast `/Game/Widgets/PopUps/SimpleToggleBox` ClickedWidget))
  (if (not (`/Game/Widgets/PopUps/SimpleToggleBox.b_IsToggleOn` _assimple_toggle_box))
    (set `self.ClickedToggle` ClickedWidget)
    (`self.ShowConfirmationPanel`)))

(event `self.ReceiveBeginPlay`
  (`self.HideConfirmationPopUp`)
  (`|ExecutionSequence`
    (:`then_0`
      ;[1 1 1] On Accept Button Pressed
      (bind _asbase_widget (cast `/Game/Widgets/PopUps/BaseWidget` (`WidgetComponent.GetUserWidgetObject` (`self.Button1`))))
      (add `/Game/Widgets/PopUps/BaseWidget.OnButtonPressed` _asbase_widget (delegate `self.OnAcceptButtonPressed`)))
    (:`then_1`
      ;[1 1 1] Storage the Widgets and Bind the Click event
      (bind _output_get (set `self.Toggles` (`|MakeArray` (`self.WidgetToggle`) (`self.WidgetToggle1`) (`self.WidgetToggle2`) (`self.WidgetToggle3`) (`self.WidgetToggle4`)))))
    (:`then_2`
      ;[1 1 1] Set Texts in Confirmation popUp
      (bind _assimple_button_text (cast `/Game/Widgets/PopUps/SimpleButtonText` (`WidgetComponent.GetUserWidgetObject` (`self.ButtonYes`)))
        (:`then`
          (`/Game/Widgets/PopUps/BaseWidget.SetText` _assimple_button_text "Si"))
        (:`CastFailed`
          _))
      (bind _assimple_button_text_2 (cast `/Game/Widgets/PopUps/SimpleButtonText` (`WidgetComponent.GetUserWidgetObject` (`self.ButtonNo`)))
        (:`then`
          (`/Game/Widgets/PopUps/BaseWidget.SetText` _assimple_button_text_2 "No"))
        (:`CastFailed`
          _))
      (bind _assimple_text_panel_widget (cast `/Game/Widgets/PopUps/SimpleTextPanelWidget` (`WidgetComponent.GetUserWidgetObject` (`self.TextConfirmation`))))
      (`/Game/Widgets/PopUps/BaseWidget.SetText` _assimple_text_panel_widget "¿Confirmas tu selección?"))
    (:`then_3`
      ;[1 1 1] Bind Confirmation Button pressed
      (bind _assimple_button_text_3 (cast `/Game/Widgets/PopUps/SimpleButtonText` (`WidgetComponent.GetUserWidgetObject` (`self.ButtonYes`)))
        (:`then`
          (add `/Game/Widgets/PopUps/BaseWidget.OnButtonPressed` _assimple_button_text_3 (delegate `OnYesButtonPressed`)))
        (:`CastFailed`
          _))
      (bind _assimple_button_text_4 (cast `/Game/Widgets/PopUps/SimpleButtonText` (`WidgetComponent.GetUserWidgetObject` (`self.ButtonNo`))))
      (add `/Game/Widgets/PopUps/BaseWidget.OnButtonPressed` _assimple_button_text_4 (delegate `OnNoButtonPressed`)))))

(event `OnYesButtonPressed`
  (params (ClickedWidget :type "/Game/Widgets/PopUps/BaseWidget Object Reference"))
  ;[1 1 1] Bind Confirmation Button pressed
  (`self.GivePoints`)
  (`self.HideConfirmationPopUp`)
  (`parent.OnAcceptButtonPressed` null))

(event `OnNoButtonPressed`
  (params (ClickedWidget :type "/Game/Widgets/PopUps/BaseWidget Object Reference"))
  ;[1 1 1] Bind Confirmation Button pressed
  (`self.HideConfirmationPopUp`))

(event `ShowConfirmationPanel`
  ;[1 1 1] Show And Hide Confirmation PopUp
  (`SceneComponent.SetRelativeScale3D` (`self.ConfirmationPopUp`) (1.0 1.0 1.0))
  (set `self.b_IsShowingConfirmationPanel` true)
  (for _array_element (`self.Toggles`)
    (`PrimitiveComponent.SetCollisionEnabled` _array_element "NoCollision")))

(event `HideConfirmationPopUp`
  ;[1 1 1] Show And Hide Confirmation PopUp
  (`SceneComponent.SetRelativeScale3D` (`self.ConfirmationPopUp`) (0.0 0.0 0.0))
  (set `self.b_IsShowingConfirmationPanel` false)
  (set `self.ClickedToggle` null)
  (for _array_element (`self.Toggles`)
    (`PrimitiveComponent.SetCollisionEnabled` _array_element "QueryOnly")))

(event `GivePoints`
  ;[1 1 1] Check the toggles and add the earned points
  (for (_array_element _array_index) (`self.Toggles`)
    (bind _asbase_widget (cast `/Game/Widgets/PopUps/BaseWidget` (`WidgetComponent.GetUserWidgetObject` _array_element)))
    (bind _assimple_toggle_box (cast `/Game/Widgets/PopUps/SimpleToggleBox` _asbase_widget))
    (if (and (not (`/Game/Widgets/PopUps/SimpleToggleBox.b_LockSelection` _assimple_toggle_box)) (`/Game/Widgets/PopUps/SimpleToggleBox.b_IsToggleOn` _assimple_toggle_box))
      (set `self.TestScore` (+ (`self.TestScore`) (`|GetArrayItem` (`self.ScoreAnswers`) _array_index))))))

(fn `GetActualToggleState`
  (returns (ActualToggleStates :type "Array of Boolean"))
  (`KismetArrayLibrary.Array_Clear` (`self.ActualToggleStates`))
  (for _array_element (`self.Toggles`)
    (bind _istoggleon (`self.GetToggleState` _array_element))
    (bind _returnvalue (`KismetArrayLibrary.Array_Add` (`self.ActualToggleStates`) _istoggleon)))
  (return (`self.ActualToggleStates`)))

(fn `GetToggleState`
  (params (ToggleBox :type "WidgetComponent Object Reference"))
  (returns (isToggleOn :type Boolean))
  (bind _assimple_toggle_box (cast `/Game/Widgets/PopUps/SimpleToggleBox` (`WidgetComponent.GetUserWidgetObject` ToggleBox)))
  (return (`/Game/Widgets/PopUps/SimpleToggleBox.b_IsToggleOn` _assimple_toggle_box)))

(fn `UserConstructionScript`
  (`parent.UserConstructionScript`))