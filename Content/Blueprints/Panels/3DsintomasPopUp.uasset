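; 3D pop-up panel for grading patient symptoms such as facial paralysis, limb paresis and agnosia, with Spanish confirmation text.
; ShowPage reveals the symptom's widget canvas and its matching toggle set, using component scale to show or hide toggles.
; Toggle presses clear their group, then after a delay recount selections against a per-page threshold.
; Enough selections open a Yes/No confirmation: Yes triggers accept, No just hides it.
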(event `self.SetupPanel`
  (params (text :type String) (b_useCancelButton :type Boolean) (pivot :type "SceneComponent Object Reference") (`Tint Color Specified Color` :type "LinearColor Structure") (Justification :type "ETextJustify Enum" :default "Left") (TextButton1 :type String) (TextButton2 :type String) (glossaryWord :type "/Game/Blueprints/Enums/GlossaryWords Enum" :default "NewEnumerator6") (OffsetSize :type "Vector2D Structure"))
  (`parent.SetupPanel` text b_useCancelButton pivot `Tint Color Specified Color` Justification TextButton1 TextButton2 glossaryWord OffsetSize))

(event `ShowPage`
  (params (Index :type Integer))
  ;[1 1 1] sHOW THE SPECIFIC PANEL
  (set `self.OpenedPage` Index)
  (bind _assintoms_calification_panel_widget (cast `/Game/Widgets/PopUps/SintomsCalificationPanelWidget` (`WidgetComponent.GetUserWidgetObject` (`self.BackgroundPanel`))))
  (switch `int` (`self.OpenedPage`)
    (:`0`
      (`Widget.SetVisibility` (`/Game/Widgets/PopUps/SintomsCalificationPanelWidget.CanvasParalisisFacil` _assintoms_calification_panel_widget) "Visible")
      (`SceneComponent.SetRelativeScale3D` (`self.Toggles2`) (0.0 0.0 0.0) :!label _label)
      (`SceneComponent.SetRelativeScale3D` (`self.Toggles3`) (0.0 0.0 0.0))
      (`SceneComponent.SetRelativeScale3D` (`self.TogglesSideSymptom2`) (0.0 0.0 0.0))
      (`SceneComponent.SetRelativeScale3D` (`self.TogglesSideSymptom`) (1.0 1.0 1.0)))
    (:`1`
      (`Widget.SetVisibility` (`/Game/Widgets/PopUps/SintomsCalificationPanelWidget.CanvasParesiaBrazo` _assintoms_calification_panel_widget) "Visible")
      (goto _label))
    (:`2`
      (`Widget.SetVisibility` (`/Game/Widgets/PopUps/SintomsCalificationPanelWidget.CanvasParesiapierna` _assintoms_calification_panel_widget) "Visible")
      (goto _label))
    (:`3`
      (`Widget.SetVisibility` (`/Game/Widgets/PopUps/SintomsCalificationPanelWidget.CanvasParalisisOcular` _assintoms_calification_panel_widget) "Visible")
      (`SceneComponent.SetRelativeScale3D` (`self.TogglesSideSymptom`) (0.0 0.0 0.0))
      (`SceneComponent.SetRelativeScale3D` (`self.Toggles3`) (0.0 0.0 0.0))
      (`SceneComponent.SetRelativeScale3D` (`self.Toggles2`) (0.0 0.0 0.0))
      (`SceneComponent.SetRelativeScale3D` (`self.TogglesSideSymptom2`) (1.0 1.0 1.0)))
    (:`4`
      (`Widget.SetVisibility` (`/Game/Widgets/PopUps/SintomsCalificationPanelWidget.CanvasParalisisAgnosia` _assintoms_calification_panel_widget) "Visible")
      (`SceneComponent.SetRelativeScale3D` (`self.TogglesSideSymptom`) (0.0 0.0 0.0))
      (`SceneComponent.SetRelativeScale3D` (`self.Toggles3`) (0.0 0.0 0.0))
      (`SceneComponent.SetRelativeScale3D` (`self.TogglesSideSymptom2`) (0.0 0.0 0.0))
      (`SceneComponent.SetRelativeScale3D` (`self.Toggles2`) (1.0 1.0 1.0)))
    (:`5`
      (`Widget.SetVisibility` (`/Game/Widgets/PopUps/SintomsCalificationPanelWidget.CanvasParalisisAgnosia2` _assintoms_calification_panel_widget) "Visible")
      (`SceneComponent.SetRelativeScale3D` (`self.Toggles2`) (0.0 0.0 0.0))
      (`SceneComponent.SetRelativeScale3D` (`self.TogglesSideSymptom`) (0.0 0.0 0.0))
      (`SceneComponent.SetRelativeScale3D` (`self.TogglesSideSymptom2`) (0.0 0.0 0.0))
      (`SceneComponent.SetRelativeScale3D` (`self.Toggles3`) (1.0 1.0 1.0)))))

(event `self.ReceiveBeginPlay`
  (`|ExecutionSequence`
    (:`then_0`
      ;[1 1 1] Set Texts in Confirmation popUp
      (bind _assimple_button_text (cast `/Game/Widgets/PopUps/SimpleButtonText` (`WidgetComponent.GetUserWidgetObject` (`self.ButtonYes`)))
        (:`then`
          (`/Game/Widgets/PopUps/BaseWidget.SetText` _assimple_button_text "Si"))
        (:`CastFailed`
          _))
      (bind _assimple_button_text_2 (cast `/Game/Widgets/PopUps/SimpleButtonText` (`WidgetComponent.GetUserWidgetObject` (`self.ButtonNo`)))
        (:`then`
          (`/Game/Widgets/PopUps/BaseWidget.SetText` _assimple_button_text_2 "No"))
        (:`CastFailed`
          _))
      (bind _assimple_text_panel_widget (cast `/Game/Widgets/PopUps/SimpleTextPanelWidget` (`WidgetComponent.GetUserWidgetObject` (`self.TextConfirmation`))))
      (`/Game/Widgets/PopUps/BaseWidget.SetText` _assimple_text_panel_widget "¿Confirmas tu selección?"))
    (:`then_1`
      ;[1 1 1] Bind confirmations popup buttons
      (bind _assimple_button_text_3 (cast `/Game/Widgets/PopUps/SimpleButtonText` (`WidgetComponent.GetUserWidgetObject` (`self.ButtonYes`)))
        (:`then`
          (add `/Game/Widgets/PopUps/BaseWidget.OnButtonPressed` _assimple_button_text_3 (delegate `OnYesButtonPressed`)))
        (:`CastFailed`
          _))
      (bind _assimple_button_text_4 (cast `/Game/Widgets/PopUps/SimpleButtonText` (`WidgetComponent.GetUserWidgetObject` (`self.ButtonNo`))))
      (add `/Game/Widgets/PopUps/BaseWidget.OnButtonPressed` _assimple_button_text_4 (delegate `OnNoButtonPressed`)))
    (:`then_2`
      ;[1 1 1] Bind Toggles
      (`|ExecutionSequence`
        (:`then_0`
          (set `self.GroupToggles3` (`|MakeArray` (`self.Toggle16`) (`self.Toggle14`) (`self.Toggle15`))))
        (:`then_1`
          (set `self.GroupToggles2` (`|MakeArray` (`self.Toggle11`) (`self.Toggle12`) (`self.Toggle13`))))
        (:`then_2`
          (set `self.GroupToggles1_1` (`|MakeArray` (`self.Toggle1`) (`self.Toggle2`))))
        (:`then_3`
          (set `self.GroupToggles1_2` (`|MakeArray` (`self.Toggle4`) (`self.Toggle3`) (`self.Toggle5`))))
        (:`then_4`
          (set `self.GroupToggles4_1` (`|MakeArray` (`self.Toggle9`) (`self.Toggle8`))))
        (:`then_5`
          (set `self.GroupToggles4_2` (`|MakeArray` (`self.Toggle6`) (`self.Toggle7`))))
        (:`then_6`
          (`|ExecutionSequence`
            (:`then_0`
              (for _array_element (`self.GroupToggles1_1`)
                (bind _assimple_toggle_box (cast `/Game/Widgets/PopUps/SimpleToggleBox` (`WidgetComponent.GetUserWidgetObject` _array_element)))
                (add `/Game/Widgets/PopUps/BaseWidget.OnButtonPressed` _assimple_toggle_box (delegate `OnToggleGroup1_1Pressed`))))
            (:`then_1`
              (for _array_element_2 (`self.GroupToggles1_2`)
                (bind _assimple_toggle_box_2 (cast `/Game/Widgets/PopUps/SimpleToggleBox` (`WidgetComponent.GetUserWidgetObject` _array_element_2)))
                (add `/Game/Widgets/PopUps/BaseWidget.OnButtonPressed` _assimple_toggle_box_2 (delegate `OnToggleGroup1_2Pressed`))))
            (:`then_2`
              (for _array_element_3 (`self.GroupToggles2`)
                (bind _assimple_toggle_box_3 (cast `/Game/Widgets/PopUps/SimpleToggleBox` (`WidgetComponent.GetUserWidgetObject` _array_element_3)))
                (add `/Game/Widgets/PopUps/BaseWidget.OnButtonPressed` _assimple_toggle_box_3 (delegate `OnToggleGroup2Pressed`))))
            (:`then_3`
              (for _array_element_4 (`self.GroupToggles3`)
                (bind _assimple_toggle_box_4 (cast `/Game/Widgets/PopUps/SimpleToggleBox` (`WidgetComponent.GetUserWidgetObject` _array_element_4)))
                (add `/Game/Widgets/PopUps/BaseWidget.OnButtonPressed` _assimple_toggle_box_4 (delegate `OnToggleGroup3Pressed`))))
            (:`then_4`
              (for _array_element_5 (`self.GroupToggles4_1`)
                (bind _assimple_toggle_box_5 (cast `/Game/Widgets/PopUps/SimpleToggleBox` (`WidgetComponent.GetUserWidgetObject` _array_element_5)))
                (add `/Game/Widgets/PopUps/BaseWidget.OnButtonPressed` _assimple_toggle_box_5 (delegate `OnToggleGroup4_1Pressed`))))
            (:`then_5`
              (for _array_element_6 (`self.GroupToggles4_2`)
                (bind _assimple_toggle_box_6 (cast `/Game/Widgets/PopUps/SimpleToggleBox` (`WidgetComponent.GetUserWidgetObject` _array_element_6)))
                (add `/Game/Widgets/PopUps/BaseWidget.OnButtonPressed` _assimple_toggle_box_6 (delegate `OnToggleGroup4_2Pressed`))))))))))

(event `OnYesButtonPressed`
  (params (ClickedWidget :type "/Game/Widgets/PopUps/BaseWidget Object Reference"))
  ;[1 1 1] Bind confirmations popup buttons
  (`self.HideConfirmationPopUp`)
  (`self.OnAcceptButtonPressed` null))

(event `OnNoButtonPressed`
  (params (ClickedWidget :type "/Game/Widgets/PopUps/BaseWidget Object Reference"))
  ;[1 1 1] Bind confirmations popup buttons
  (`self.HideConfirmationPopUp`))

(event `OnToggleGroup1_1Pressed`
  (params (ClickedWidget :type "/Game/Widgets/PopUps/BaseWidget Object Reference"))
  ;[1 1 1] Bind Toggles
  (for _array_element (`self.GroupToggles1_1`)
    (bind _assimple_toggle_box (cast `/Game/Widgets/PopUps/SimpleToggleBox` (`WidgetComponent.GetUserWidgetObject` _array_element)))
    (`/Game/Widgets/PopUps/SimpleToggleBox.SetToggleValue` _assimple_toggle_box false))
  (`KismetSystemLibrary.Delay` 0.2)
  (`self.UpdateToggles`))

(event `UpdateToggles`
  (set `self.selectedToggles` 0)
  (`|ExecutionSequence`
    (:`then_0`
      (for _array_element (`self.GroupToggles3`)
        (bind _assimple_toggle_box (cast `/Game/Widgets/PopUps/SimpleToggleBox` (`WidgetComponent.GetUserWidgetObject` _array_element)))
        (if (`/Game/Widgets/PopUps/SimpleToggleBox.b_IsToggleOn` _assimple_toggle_box)
          (`/Engine/EditorBlueprintResources/StandardMacros.IncrementInt` (`self.selectedToggles`) :!label _label_2))))
    (:`then_1`
      (for _array_element_2 (`self.GroupToggles2`)
        (bind _assimple_toggle_box_2 (cast `/Game/Widgets/PopUps/SimpleToggleBox` (`WidgetComponent.GetUserWidgetObject` _array_element_2)))
        (if (`/Game/Widgets/PopUps/SimpleToggleBox.b_IsToggleOn` _assimple_toggle_box_2)
          (goto _label_2))))
    (:`then_2`
      (for _array_element_3 (`self.GroupToggles1_1`)
        (bind _assimple_toggle_box_3 (cast `/Game/Widgets/PopUps/SimpleToggleBox` (`WidgetComponent.GetUserWidgetObject` _array_element_3)))
        (if (`/Game/Widgets/PopUps/SimpleToggleBox.b_IsToggleOn` _assimple_toggle_box_3)
          (goto _label_2))))
    (:`then_3`
      (for _array_element_4 (`self.GroupToggles1_2`)
        (bind _assimple_toggle_box_4 (cast `/Game/Widgets/PopUps/SimpleToggleBox` (`WidgetComponent.GetUserWidgetObject` _array_element_4)))
        (if (`/Game/Widgets/PopUps/SimpleToggleBox.b_IsToggleOn` _assimple_toggle_box_4)
          (goto _label_2))))
    (:`then_4`
      (for _array_element_5 (`self.GroupToggles4_1`)
        (bind _assimple_toggle_box_5 (cast `/Game/Widgets/PopUps/SimpleToggleBox` (`WidgetComponent.GetUserWidgetObject` _array_element_5)))
        (if (`/Game/Widgets/PopUps/SimpleToggleBox.b_IsToggleOn` _assimple_toggle_box_5)
          (goto _label_2))))
    (:`then_5`
      (for _array_element_6 (`self.GroupToggles4_2`)
        (bind _assimple_toggle_box_6 (cast `/Game/Widgets/PopUps/SimpleToggleBox` (`WidgetComponent.GetUserWidgetObject` _array_element_6)))
        (if (`/Game/Widgets/PopUps/SimpleToggleBox.b_IsToggleOn` _assimple_toggle_box_6)
          (goto _label_2))))
    (:`then_6`
      (`KismetSystemLibrary.Delay` 0.2)
      (if (> (`self.selectedToggles`) (select `int` (`self.OpenedPage`) :`0` 1 :`1` 1 :`2` 1 :`3` 1 :`4` 0 :`5` 0))
        (`self.FinishSelection`)))))

(event `FinishSelection`
  (`self.ShowConfirmationPanel`))

(event `ShowConfirmationPanel`
  (`SceneComponent.SetRelativeScale3D` (`self.ConfirmationPopUp`) (1.0 1.0 1.0)))

(event `OnToggleGroup1_2Pressed`
  (params (ClickedWidget :type "/Game/Widgets/PopUps/BaseWidget Object Reference"))
  ;[1 1 1] Bind Toggles
  (for _array_element (`self.GroupToggles1_2`)
    (bind _assimple_toggle_box (cast `/Game/Widgets/PopUps/SimpleToggleBox` (`WidgetComponent.GetUserWidgetObject` _array_element)))
    (`/Game/Widgets/PopUps/SimpleToggleBox.SetToggleValue` _assimple_toggle_box false))
  (`KismetSystemLibrary.Delay` 0.2)
  (`self.UpdateToggles`))

(event `HideConfirmationPopUp`
  (`SceneComponent.SetRelativeScale3D` (`self.ConfirmationPopUp`) (0.0 0.0 0.0)))

(event `OnToggleGroup2Pressed`
  (params (ClickedWidget :type "/Game/Widgets/PopUps/BaseWidget Object Reference"))
  ;[1 1 1] Bind Toggles
  (for _array_element (`self.GroupToggles2`)
    (bind _assimple_toggle_box (cast `/Game/Widgets/PopUps/SimpleToggleBox` (`WidgetComponent.GetUserWidgetObject` _array_element)))
    (`/Game/Widgets/PopUps/SimpleToggleBox.SetToggleValue` _assimple_toggle_box false))
  (`KismetSystemLibrary.Delay` 0.2)
  (`self.UpdateToggles`))

(event `OnToggleGroup3Pressed`
  (params (ClickedWidget :type "/Game/Widgets/PopUps/BaseWidget Object Reference"))
  ;[1 1 1] Bind Toggles
  (for _array_element (`self.GroupToggles3`)
    (bind _assimple_toggle_box (cast `/Game/Widgets/PopUps/SimpleToggleBox` (`WidgetComponent.GetUserWidgetObject` _array_element)))
    (`/Game/Widgets/PopUps/SimpleToggleBox.SetToggleValue` _assimple_toggle_box false))
  (`KismetSystemLibrary.Delay` 0.2)
  (`self.UpdateToggles`))

(event `OnToggleGroup4_1Pressed`
  (params (ClickedWidget :type "/Game/Widgets/PopUps/BaseWidget Object Reference"))
  ;[1 1 1] Bind Toggles
  (for _array_element (`self.GroupToggles4_1`)
    (bind _assimple_toggle_box (cast `/Game/Widgets/PopUps/SimpleToggleBox` (`WidgetComponent.GetUserWidgetObject` _array_element)))
    (`/Game/Widgets/PopUps/SimpleToggleBox.SetToggleValue` _assimple_toggle_box false))
  (`KismetSystemLibrary.Delay` 0.2)
  (`self.UpdateToggles`))

(event `OnToggleGroup4_2Pressed`
  (params (ClickedWidget :type "/Game/Widgets/PopUps/BaseWidget Object Reference"))
  ;[1 1 1] Bind Toggles
  (for _array_element (`self.GroupToggles4_2`)
    (bind _assimple_toggle_box (cast `/Game/Widgets/PopUps/SimpleToggleBox` (`WidgetComponent.GetUserWidgetObject` _array_element)))
    (`/Game/Widgets/PopUps/SimpleToggleBox.SetToggleValue` _assimple_toggle_box false))
  (`KismetSystemLibrary.Delay` 0.2)
  (`self.UpdateToggles`))

(fn `UserConstructionScript`
  (`parent.UserConstructionScript`))