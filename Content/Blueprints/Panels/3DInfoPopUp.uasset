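; 3DInfoPopUp is a 3D panel actor with two widget-component buttons that show point feedback for correct and wrong answers.
; Two events take the earned points and a button index, cast that button's widget to SimpleButtonText and play its points animation, green for correct and red for wrong.
; BeginPlay and construction only call the parent, and SetOffsetSize is empty.
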(event `self.ReceiveBeginPlay`
  (`parent.ReceiveBeginPlay`))

(event `PlayCorrectAnswerAnimation`
  (params (EarnedPoints :type Integer) (IndexButtonToAnim :type Integer))
  (switch `int` IndexButtonToAnim
    (:`0`
      (bind _assimple_button_text (cast `/Game/Widgets/PopUps/SimpleButtonText` (`WidgetComponent.GetUserWidgetObject` (`self.Button1`))))
      (`/Game/Widgets/PopUps/SimpleButtonText.PlayPointsAnimation` _assimple_button_text EarnedPoints (struct :`R` 0.473532 :`G` 0.799103 :`B` 0.14996 :`A` 1.0)))
    (:`1`
      (bind _assimple_button_text_2 (cast `/Game/Widgets/PopUps/SimpleButtonText` (`WidgetComponent.GetUserWidgetObject` (`self.Button2`))))
      (`/Game/Widgets/PopUps/SimpleButtonText.PlayPointsAnimation` _assimple_button_text_2 EarnedPoints (struct :`R` 0.473532 :`G` 0.799103 :`B` 0.14996 :`A` 1.0)))))

(event `PlayWrongAnswerAnimation`
  (params (EarnedPoints :type Integer) (IndexButtonToAnim :type Integer))
  (switch `int` IndexButtonToAnim
    (:`0`
      (bind _assimple_button_text (cast `/Game/Widgets/PopUps/SimpleButtonText` (`WidgetComponent.GetUserWidgetObject` (`self.Button1`))))
      (`/Game/Widgets/PopUps/SimpleButtonText.PlayPointsAnimation` _assimple_button_text EarnedPoints (struct :`R` 0.991102 :`G` 0.181165 :`B` 0.181165 :`A` 1.0)))
    (:`1`
      (bind _assimple_button_text_2 (cast `/Game/Widgets/PopUps/SimpleButtonText` (`WidgetComponent.GetUserWidgetObject` (`self.Button2`))))
      (`/Game/Widgets/PopUps/SimpleButtonText.PlayPointsAnimation` _assimple_button_text_2 EarnedPoints (struct :`R` 0.991102 :`G` 0.181165 :`B` 0.181165 :`A` 1.0)))))

(event `self.SetOffsetSize`
  (params (Size :type "Vector2D Structure")))

(fn `UserConstructionScript`
  (`parent.UserConstructionScript`))