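; Child 3D pop-up panel for "Cincinnati" with three widget toggles and an accept button, extending a parent panel's setup and accept logic.
; BeginPlay binds Button1 to accept, enables input, sets widget interaction references and starts a fast looping UpdateRotation timer.
; SetupPanel forwards to the parent, then shrinks the actor's scale.
; GetActualToggleState reads SimpleToggleBox states into an array, but returns inside the loop body.
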(event `self.OnAcceptButtonPressed`
  (params (ClickedWidget :type "/Game/Widgets/PopUps/BaseWidget Object Reference"))
  (`parent.OnAcceptButtonPressed` null))

(event `self.ReceiveBeginPlay`
  (`|ExecutionSequence`
    (:`then_0`
      (set `self.Toggles` (`|MakeArray` (`self.WidgetToggle`) (`self.WidgetToggle1`) (`self.WidgetToggle2`)))
      (bind _asbase_widget (cast `/Game/Widgets/PopUps/BaseWidget` (`WidgetComponent.GetUserWidgetObject` (`self.Button1`))))
      (add `/Game/Widgets/PopUps/BaseWidget.OnButtonPressed` _asbase_widget (delegate `self.OnAcceptButtonPressed`)))
    (:`then_1`
      (`self.EnableInput` (`GameplayStatics.GetPlayerController` 0))
      (`self.SetWidgetInteractionReferences`)
      (`self.GetGameManager`)
      (`KismetSystemLibrary.K2_SetTimer` null "UpdateRotation" 0.001 true))))

(event `self.SetupPanel`
  (params (text :type String) (b_useCancelButton :type Boolean) (pivot :type "SceneComponent Object Reference") (`Tint Color Specified Color` :type "LinearColor Structure") (Justification :type "ETextJustify Enum" :default "Left") (TextButton1 :type String) (TextButton2 :type String) (glossaryWord :type "/Game/Blueprints/Enums/GlossaryWords Enum" :default "NewEnumerator6") (OffsetSize :type "Vector2D Structure"))
  (`parent.SetupPanel` text b_useCancelButton pivot `Tint Color Specified Color` Justification TextButton1 TextButton2 glossaryWord OffsetSize)
  (`self.SetActorScale3D` (0.23 0.23 0.23)))

(fn `GetActualToggleState`
  (returns (ActualToggleStates :type "Array of Boolean"))
  (bind _actualtogglestates (`self.ActualToggleStates`))
  (for (_array_element _array_index) (`self.Toggles`)
    (bind _istoggleon (`self.GetToggleState` _array_element))
    (`KismetArrayLibrary.Array_Set` _actualtogglestates _array_index _istoggleon true)
    (return _actualtogglestates)))

(fn `GetToggleState`
  (params (ToggleBox :type "WidgetComponent Object Reference"))
  (returns (isToggleOn :type Boolean))
  (bind _assimple_toggle_box (cast `/Game/Widgets/PopUps/SimpleToggleBox` (`WidgetComponent.GetUserWidgetObject` ToggleBox)))
  (return (`/Game/Widgets/PopUps/SimpleToggleBox.b_IsToggleOn` _assimple_toggle_box)))

(fn `UserConstructionScript`
  (`parent.UserConstructionScript`))