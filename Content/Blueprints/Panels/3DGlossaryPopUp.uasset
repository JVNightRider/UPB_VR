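; 3D glossary pop-up panel that shows text and can open a nested glossary word when tapped.
; SetupPanel override fills text, buttons, color and layout, and scales the actor down.
; With a glossary word, text taps notify SceneFlowManager through GameManager and are also bound to accept.
; Background taps trigger the parent's accept handler, as do text taps without a word; BeginPlay skips its parent call.
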(event `OnInsideGlosaryTapped`
  (params (ClickedWidget :type "/Game/Widgets/PopUps/BaseWidget Object Reference"))
  ;[1 1 1] Detect glossary Text Tapped
  (`/Game/Blueprints/Managers/SceneFlowManager.InternalGlossaryWordTapped` (`/Game/Blueprints/Managers/GameManager.SceneFlowManager` (`self.GameManager`)) (`self.glossaryWord`) self))

(event `self.SetupPanel`
  (params (text :type String) (b_useCancelButton :type Boolean) (pivot :type "SceneComponent Object Reference") (`Tint Color Specified Color` :type "LinearColor Structure") (Justification :type "ETextJustify Enum" :default "Left") (TextButton1 :type String) (TextButton2 :type String) (glossaryWord :type "/Game/Blueprints/Enums/GlossaryWords Enum" :default "NewEnumerator6") (OffsetSize :type "Vector2D Structure"))
  ;[1 1 1] Override Setup Panel to add the text detection in case of have some glossary word
  (bind _asbase_widget (cast `/Game/Widgets/PopUps/BaseWidget` (`WidgetComponent.GetUserWidgetObject` (`self.Text`)))
    (:`then`
      (`/Game/Widgets/PopUps/BaseWidget.SetText` _asbase_widget text))
    (:`CastFailed`
      _))
  (`SceneComponent.SetVisibility` (`self.Button2`) b_useCancelButton false)
  (`self.SetActorScale3D` (0.1 0.1 0.1))
  (`self.SetColorPanel` `Tint Color Specified Color`)
  (`self.SetJustification` Justification)
  (`self.SetButton1Text` TextButton1)
  (`self.SetButton2Text` TextButton2)
  (`self.SetOffsetSize` OffsetSize)
  (bind _output_get (set `self.glossaryWord` glossaryWord))
  (if (`|EnumInequality` _output_get "NewEnumerator6")
    (bind _asbase_widget_2 (cast `/Game/Widgets/PopUps/BaseWidget` (`WidgetComponent.GetUserWidgetObject` (`self.Text`))))
    (add `/Game/Widgets/PopUps/BaseWidget.OnButtonPressed` _asbase_widget_2 (delegate `OnInsideGlosaryTapped`))
    (bind _asbase_widget_3 (cast `/Game/Widgets/PopUps/BaseWidget` (`WidgetComponent.GetUserWidgetObject` (`self.Text`))))
    (add `/Game/Widgets/PopUps/BaseWidget.OnButtonPressed` _asbase_widget_3 (delegate `self.OnAcceptButtonPressed`))
    (else
      (bind _asbase_widget_4 (cast `/Game/Widgets/PopUps/BaseWidget` (`WidgetComponent.GetUserWidgetObject` (`self.Text`))))
      (bind _asbase_widget_5 (cast `/Game/Widgets/PopUps/BaseWidget` (`WidgetComponent.GetUserWidgetObject` (`self.BackgroundPanel`))))
      (add `/Game/Widgets/PopUps/BaseWidget.OnButtonPressed` _asbase_widget_5 (delegate `self.OnAcceptButtonPressed`))
      (add `/Game/Widgets/PopUps/BaseWidget.OnButtonPressed` _asbase_widget_4 (delegate `self.OnAcceptButtonPressed`)))))

(event `self.OnAcceptButtonPressed`
  (params (ClickedWidget :type "/Game/Widgets/PopUps/BaseWidget Object Reference"))
  ;[1 1 1] If click background text trigger accept button Call
  (`parent.OnAcceptButtonPressed` ClickedWidget))

(event `self.ReceiveBeginPlay`
  ;[1 1 1] If click background text trigger accept button Call
  (bind _asbase_widget (cast `/Game/Widgets/PopUps/BaseWidget` (`WidgetComponent.GetUserWidgetObject` (`self.BackgroundPanel`))))
  (add `/Game/Widgets/PopUps/BaseWidget.OnButtonPressed` _asbase_widget (delegate `self.OnAcceptButtonPressed`)))

(fn `UserConstructionScript`
  (`parent.UserConstructionScript`))