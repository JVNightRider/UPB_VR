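; 3D pop-up panel actor for the SEM call, with two answer buttons and two glossary text widgets.
; On BeginPlay it binds the widgets' press events, gets the game manager and starts a looping UpdateRotation timer.
; Button presses set flags, while text taps send the ACV or SEM glossary word to the SceneFlowManager.
; Answer events play a green or red points animation on the indexed button.
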(event `PlayCorrectAnswerAnimation`
  (params (EarnedPoints :type Integer) (IndexButtonToAnim :type Integer))
  (switch `int` IndexButtonToAnim
    (:`0`
      (bind _assimple_button_text (cast `/Game/Widgets/PopUps/SimpleButtonText` (`WidgetComponent.GetUserWidgetObject` (`self.Button1`))))
      (`/Game/Widgets/PopUps/SimpleButtonText.PlayPointsAnimation` _assimple_button_text EarnedPoints (struct :`R` 0.473532 :`G` 0.799103 :`B` 0.14996 :`A` 1.0)))
    (:`1`
      (bind _assimple_button_text_2 (cast `/Game/Widgets/PopUps/SimpleButtonText` (`WidgetComponent.GetUserWidgetObject` (`self.Button2`))))
      (`/Game/Widgets/PopUps/SimpleButtonText.PlayPointsAnimation` _assimple_button_text_2 EarnedPoints (struct :`R` 0.473532 :`G` 0.799103 :`B` 0.14996 :`A` 1.0)))))

(event `PlayWrongAnswerAnimation`
  (params (EarnedPoints :type Integer) (IndexButtonToAnim :type Integer))
  (switch `int` IndexButtonToAnim
    (:`0`
      (bind _assimple_button_text (cast `/Game/Widgets/PopUps/SimpleButtonText` (`WidgetComponent.GetUserWidgetObject` (`self.Button1`))))
      (`/Game/Widgets/PopUps/SimpleButtonText.PlayPointsAnimation` _assimple_button_text EarnedPoints (struct :`R` 0.991102 :`G` 0.181165 :`B` 0.181165 :`A` 1.0)))
    (:`1`
      (bind _assimple_button_text_2 (cast `/Game/Widgets/PopUps/SimpleButtonText` (`WidgetComponent.GetUserWidgetObject` (`self.Button2`))))
      (`/Game/Widgets/PopUps/SimpleButtonText.PlayPointsAnimation` _assimple_button_text_2 EarnedPoints (struct :`R` 0.991102 :`G` 0.181165 :`B` 0.181165 :`A` 1.0)))))

(event `CustomEvent_2`
  (params (ClickedWidget :type "/Game/Widgets/PopUps/BaseWidget Object Reference"))
  ;[1 1 1] Detect Accept And Cancel Buttons pressed
  (set `self.isButton1Pressed` true))

(event `OpenACVGlossary`
  (params (ClickedWidget :type "/Game/Widgets/PopUps/BaseWidget Object Reference"))
  ;[1 1 1] Detect glossary Text Tapped
  (`/Game/Blueprints/Managers/SceneFlowManager.GlossaryWordTaped` (`/Game/Blueprints/Managers/GameManager.SceneFlowManager` (`self.GameManager`)) "NewEnumerator4" self))

(event `OpenSEMGlossary`
  (params (ClickedWidget :type "/Game/Widgets/PopUps/BaseWidget Object Reference"))
  ;[1 1 1] Detect glossary Text Tapped
  (`/Game/Blueprints/Managers/SceneFlowManager.GlossaryWordTaped` (`/Game/Blueprints/Managers/GameManager.SceneFlowManager` (`self.GameManager`)) "NewEnumerator5" self))

(event `CustomEvent_1`
  (params (ClickedWidget :type "/Game/Widgets/PopUps/BaseWidget Object Reference"))
  ;[1 1 1] Detect Accept And Cancel Buttons pressed
  (set `self.isButton2Pressed` true))

(event `self.ReceiveBeginPlay`
  (`|ExecutionSequence`
    (:`then_0`
      (bind _asbase_widget (cast `/Game/Widgets/PopUps/BaseWidget` (`WidgetComponent.GetUserWidgetObject` (`self.Button1`)))
        (:`then`
          (add `/Game/Widgets/PopUps/BaseWidget.OnButtonPressed` _asbase_widget (delegate `CustomEvent_2`)))
        (:`CastFailed`
          _))
      (bind _asbase_widget_2 (cast `/Game/Widgets/PopUps/BaseWidget` (`WidgetComponent.GetUserWidgetObject` (`self.Button2`)))
        (:`then`
          (add `/Game/Widgets/PopUps/BaseWidget.OnButtonPressed` _asbase_widget_2 (delegate `CustomEvent_1`)))
        (:`CastFailed`
          _))
      (bind _asbase_widget_3 (cast `/Game/Widgets/PopUps/BaseWidget` (`WidgetComponent.GetUserWidgetObject` (`self.Text1`))))
      (add `/Game/Widgets/PopUps/BaseWidget.OnButtonPressed` _asbase_widget_3 (delegate `OpenACVGlossary`))
      (bind _asbase_widget_4 (cast `/Game/Widgets/PopUps/BaseWidget` (`WidgetComponent.GetUserWidgetObject` (`self.Text2`))))
      (add `/Game/Widgets/PopUps/BaseWidget.OnButtonPressed` _asbase_widget_4 (delegate `OpenSEMGlossary`)))
    (:`then_1`
      (`self.EnableInput` (`GameplayStatics.GetPlayerController` 0))
      (`self.SetWidgetInteractionReferences`)
      (`self.GetGameManager`)
      (`KismetSystemLibrary.K2_SetTimer` null "UpdateRotation" 0.001 true))))

(fn `UserConstructionScript`
  (`parent.UserConstructionScript`))