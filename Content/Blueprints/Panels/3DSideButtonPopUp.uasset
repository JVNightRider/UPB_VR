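; A 3D side-button pop-up panel actor whose Button1 widget component displays a SideButtonColor user widget.
; SetColorPanel casts that widget and passes it a tint color through SetPanelColor.
; SetOffsetSize runs the parent's version, then adds the given size to Button1's current draw size, so repeated calls accumulate.
; BeginPlay and construction only defer to the parent class.
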(event `self.SetColorPanel`
  (params (`Tint Color Specified Color` :type "LinearColor Structure"))
  (bind _asside_button_color (cast `/Game/Widgets/PopUps/SideButtonColor` (`WidgetComponent.GetUserWidgetObject` (`self.Button1`))))
  (`/Game/Widgets/PopUps/SideButtonColor.SetPanelColor` _asside_button_color `Tint Color Specified Color`))

(event `self.ReceiveBeginPlay`
  (`parent.ReceiveBeginPlay`))

(event `self.SetOffsetSize`
  (params (Size :type "Vector2D Structure"))
  (bind _button1 (`self.Button1`))
  (`parent.SetOffsetSize` Size)
  (`WidgetComponent.SetDrawSize` _button1 (+ Size (`WidgetComponent.GetDrawSize` _button1))))

(fn `UserConstructionScript`
  (`parent.UserConstructionScript`))