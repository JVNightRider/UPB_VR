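; A 3D dialog pop-up panel that shows a character face beside a colorable button, built from widget components.
; SetCharacterImage looks up the character name in the CharacterFaces data table and passes the row's image to the face widget.
; SetColorPanel tints the button's panel and keeps its arrow white.
; SetOffsetSize extends the parent's resizing by adding the offset to the button's draw size.
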(event `self.SetColorPanel`
  (params (`Tint Color Specified Color` :type "LinearColor Structure"))
  (bind _asside_button_color (cast `/Game/Widgets/PopUps/SideButtonColor` (`WidgetComponent.GetUserWidgetObject` (`self.Button1`))))
  (`/Game/Widgets/PopUps/SideButtonColor.SetPanelColor` _asside_button_color `Tint Color Specified Color`)
  (`Image.SetBrushTintColor` (`/Game/Widgets/PopUps/SideButtonColor.Image_Arrow` _asside_button_color) (make `SlateColor` (struct :`R` 1.0 :`G` 1.0 :`B` 1.0 :`A` 1.0))))

(event `self.ReceiveBeginPlay`
  (`parent.ReceiveBeginPlay`))

(event `SetCharacterImage`
  (params (CharacterName :type Name :default "Martha"))
  (bind _returnvalue (`|GetDataTableRow` "/Game/DataTables/CharacterFacesDataTable.CharacterFacesDataTable" CharacterName)
    (:`then`
      (bind _assimple_image_widget (cast `/Game/Widgets/PopUps/SimpleImageWidget` (`WidgetComponent.GetUserWidgetObject` (`self.CharacterFace`))))
      (`/Game/Widgets/PopUps/SimpleImageWidget.SetTextureImage` _assimple_image_widget (break `/Game/DataTables/CharacterFacesStructure` _returnvalue)))))

(event `self.SetOffsetSize`
  (params (Size :type "Vector2D Structure"))
  (bind _button1 (`self.Button1`))
  (`parent.SetOffsetSize` Size)
  (`WidgetComponent.SetDrawSize` _button1 (+ Size (`WidgetComponent.GetDrawSize` _button1))))

(fn `UserConstructionScript`
  (`parent.UserConstructionScript`))