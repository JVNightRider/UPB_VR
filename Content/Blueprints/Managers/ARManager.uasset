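; AR manager that tracks the active scene object and routes screen taps to widgets placed in the world.
; Setting a new scene object fires a change dispatcher, notifies SceneFlowManager and starts looping touch polling until FinishScene clears it.
; Each poll deprojects the touch into a line trace and calls ButtonClicked on any visible BaseWidget hit, repeating while held.
; It also supplies the object class for the current scene index.
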(event `self.ReceiveBeginPlay`
  (`parent.ReceiveBeginPlay`))

(event `SetNewSceneObject`
  (params (newSceneObject :type "/Game/Blueprints/SceneObjects/BP_SceneObject Object Reference"))
  (set `self.actualSceneObject` newSceneObject)
  (`self.OnSceneObjectChange`)
  (`/Game/Blueprints/Managers/SceneFlowManager.OnNewSceneObjectDetected` (`/Game/Blueprints/Managers/GameManager.SceneFlowManager` (`self.GameManager`)))
  (bind _returnvalue (`KismetSystemLibrary.K2_SetTimer` null "GetTouch" 0.01 true))
  (set `self.TouchTimer` _returnvalue))

(event `FinishScene`
  (`KismetSystemLibrary.K2_ClearAndInvalidateTimerHandle` (`self.TouchTimer`)))

(fn `GetSceneObjectClass`
  (returns (NewParam :type "/Game/Blueprints/SceneObjects/BP_SceneObject Class Reference"))
  (return (`|GetArrayItem` (`self.AllSceneObjects`) (`/Game/Blueprints/Managers/SceneFlowManager.actualSceneIndex` (`/Game/Blueprints/Managers/GameManager.SceneFlowManager` (`self.GameManager`))))))

(fn `GetTouch`
  (bind (_location _ispressed) (`self.GetTouchLocation`))
  (if _ispressed
    (bind (_hitinfo _returnvalue) (`self.WorldHitTest` _location))
    (bind (_bblockinghit _binitialoverlap _time _distance _location_2 _impactpoint _normal _impactnormal _physmat _hitactor _hitcomponent) (`GameplayStatics.BreakHitResult` _hitinfo))
    (`/Engine/EditorBlueprintResources/StandardMacros.IsValid` _hitcomponent
      (:`Is Valid`
        (if (and _returnvalue (not (`Actor.bHidden` _hitactor)) (`self.IsVisible` _hitcomponent))
          (bind _aswidget_component (cast `WidgetComponent` _hitcomponent))
          (bind _asbase_widget (cast `/Game/Widgets/PopUps/BaseWidget` (`WidgetComponent.GetWidget` _aswidget_component)))
          (`/Game/Widgets/PopUps/TestWidget.ButtonClicked` _asbase_widget))))))

(fn `GetTouchLocation`
  (returns (Location :type "Vector2D Structure") (isPressed :type Boolean))
  (bind (_locationx _locationy _biscurrentlypressed) (`PlayerController.GetInputTouchState` (`GameplayStatics.GetPlayerController` 0) "Touch1"))
  (return (`KismetMathLibrary.MakeVector2D` _locationx _locationy) _biscurrentlypressed))

(fn `WorldHitTest`
  (params (TouchLocation :type "Vector2D Structure"))
  (returns (HitInfo :type "HitResult Structure") (ReturnValue :type Boolean))
  (bind (_worldposition _worlddirection) (`GameplayStatics.DeprojectScreenToWorld` (`GameplayStatics.GetPlayerController` 0) TouchLocation))
  (bind (_outhit _returnvalue) (`KismetSystemLibrary.LineTraceSingleForObjects` :`Start` _worldposition :`End` (+ _worldposition (* _worlddirection 1000.0)) :`ObjectTypes` (`|MakeArray` "ObjectTypeQuery1" "ObjectTypeQuery2" "ObjectTypeQuery3" "ObjectTypeQuery4" "ObjectTypeQuery5" "ObjectTypeQuery6" :!type "EObjectTypeQuery Enum") :`bIgnoreSelf` false))
  (return _outhit _returnvalue))