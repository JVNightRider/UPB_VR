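; Manager that spawns the game's 3D pop-up panels (info, dialog, glossary and medical-themed ones like Cincinnati and symptoms) and relays their input.
; Each Show function spawns its panel class at a pivot's transform, configures it through SetupPanel and returns the actor.
; Button presses fire Accept/Cancel dispatchers and briefly raise polled-style flags, with a Gate blocking repeats during the short delay.
; Option selections are rebroadcast, and FinishScene resets toggle answers.
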(event `self.ReceiveBeginPlay`
  (`parent.ReceiveBeginPlay`))

(event `ButtonPressed`
  (params (ButtonType :type "/Game/Blueprints/Enums/ButtonType Enum" :default "NewEnumerator0"))
  ;[0 0 0] Detects the input from the panels
  (`|ExecutionSequence`
    (:`then_0`
      (`/Engine/EditorBlueprintResources/StandardMacros.Gate` false :!label _label
        (:`Exit`
          (switch `/Game/Blueprints/Enums/ButtonType` ButtonType
            (:`NewEnumerator1`
              (set `self.b_IsAcceptButtonPressed` true)
              (`self.OnAceptButtonPressed`)
              (`KismetSystemLibrary.Delay` 0.2)
              (set `self.b_IsAcceptButtonPressed` false)
              (goto _label :!via `Open`))
            (:`NewEnumerator0`
              (set `self.b_IsCancelButtonPressed` true)
              (`self.OnCancelButtonPressed`)
              (`KismetSystemLibrary.Delay` 0.2)
              (set `self.b_IsCancelButtonPressed` false)
              (goto _label :!via `Open`))))))
    (:`then_1`
      (goto _label :!via `Close`))))

(event `OptionSelected`
  (params (indexOption :type Integer))
  (`self.OnSelectedOption` indexOption))

(event `self.FinishScene`
  (`self.ClearToggleAnswers`))

(event `ClearToggleAnswers`
  (set `self.ToggleAnswers` (`|MakeArray` false)))

(fn `Show Dialog Pop Up Panel`
  (params (pivot :type "SceneComponent Object Reference") (text :type String) (`Tint Color Specified Color` :type "LinearColor Structure") (Justification :type "ETextJustify Enum" :default "Left") (glossaryWord :type "/Game/Blueprints/Enums/GlossaryWords Enum" :default "NewEnumerator6") (CharacterName :type Name) (OffsetSize :type "Vector2D Structure"))
  (returns (createdPanel :type "/Game/Blueprints/Panels/3DPanel Object Reference"))
  (bind _returnvalue (`|SpawnActorFromClass` (`self.DialogPopUpPrefab`) (`self.K2_GetComponentToWorld` pivot) "Undefined" "OverrideRootScale" null null))
  (bind _as3dpanel (cast `/Game/Blueprints/Panels/3DPanel` _returnvalue))
  (`/Game/Blueprints/Panels/3DPanel.SetupPanel` _as3dpanel text false pivot `Tint Color Specified Color` Justification "" "" glossaryWord OffsetSize)
  (bind _as3ddialog_pop_up (cast `/Game/Blueprints/Panels/3DDialogPopUp` _returnvalue))
  (`/Game/Blueprints/Panels/3DDialogPopUp.SetCharacterImage` _as3ddialog_pop_up CharacterName)
  (return _returnvalue))

(fn `ShowBeFastPanel`
  (params (pivot :type "SceneComponent Object Reference") (text :type String) (`Tint Color Specified Color` :type "LinearColor Structure") (Justification :type "ETextJustify Enum" :default "Left") (glossaryWord :type "/Game/Blueprints/Enums/GlossaryWords Enum" :default "NewEnumerator6") (OffsetSize :type "Vector2D Structure"))
  (returns (createdPanel :type "/Game/Blueprints/Panels/3DPanel Object Reference"))
  (bind _returnvalue (`|SpawnActorFromClass` (`self.BeFastPopUpPrefab`) (`self.K2_GetComponentToWorld` pivot) "Undefined" "OverrideRootScale" null null))
  (bind _as3dpanel (cast `/Game/Blueprints/Panels/3DPanel` _returnvalue))
  (`/Game/Blueprints/Panels/3DPanel.SetupPanel` _as3dpanel text false pivot `Tint Color Specified Color` Justification "Confirmar" "" glossaryWord OffsetSize)
  (return _returnvalue))

(fn `ShowButtonlessPopUpPanel`
  (params (pivot :type "SceneComponent Object Reference") (text :type String) (`Tint Color Specified Color` :type "LinearColor Structure") (Justification :type "ETextJustify Enum" :default "Center") (OffsetSize :type "Vector2D Structure"))
  (returns (createdPanel :type "/Game/Blueprints/Panels/3DPanel Object Reference"))
  (bind _returnvalue (`|SpawnActorFromClass` (`self.ButtonLessPopUpPrefab`) (`self.K2_GetComponentToWorld` pivot) "Undefined" "OverrideRootScale" null null))
  (bind _as3dpanel (cast `/Game/Blueprints/Panels/3DPanel` _returnvalue))
  (`/Game/Blueprints/Panels/3DPanel.SetupPanel` _as3dpanel text false pivot `Tint Color Specified Color` Justification "" "" "NewEnumerator6" OffsetSize)
  (return _returnvalue))

(fn `ShowButtonSideColorPanel`
  (params (pivot :type "SceneComponent Object Reference") (text :type String) (`Tint Color Specified Color` :type "LinearColor Structure") (Justification :type "ETextJustify Enum" :default "Left") (glossaryWord :type "/Game/Blueprints/Enums/GlossaryWords Enum" :default "NewEnumerator6") (OffsetSize :type "Vector2D Structure"))
  (returns (createdPanel :type "/Game/Blueprints/Panels/3DPanel Object Reference"))
  (bind _returnvalue (`|SpawnActorFromClass` (`self.ButtonSideColorPanel`) (`self.K2_GetComponentToWorld` pivot) "Undefined" "OverrideRootScale" null null))
  (bind _as3dpanel (cast `/Game/Blueprints/Panels/3DPanel` _returnvalue))
  (`/Game/Blueprints/Panels/3DPanel.SetupPanel` _as3dpanel text false pivot `Tint Color Specified Color` Justification "" "" glossaryWord OffsetSize)
  (return _returnvalue))

(fn `ShowCallSEMPanel`
  (params (pivot :type "SceneComponent Object Reference"))
  (returns (createdPanel :type "/Game/Blueprints/Panels/3DPanel Object Reference"))
  (bind _returnvalue (`|SpawnActorFromClass` (`self.CallSEMPopUpPrefab`) (`self.K2_GetComponentToWorld` pivot) "Undefined" "OverrideRootScale" null null))
  (bind _as3dpanel (cast `/Game/Blueprints/Panels/3DPanel` _returnvalue))
  (`/Game/Blueprints/Panels/3DPanel.SetupPanel` _as3dpanel "" true pivot (struct :`R` 1.0 :`G` 1.0 :`B` 1.0 :`A` 1.0) "Left" "" "" "NewEnumerator6" (0.0 0.0))
  (return _returnvalue))

(fn `ShowCincinnatiPanel`
  (params (pivot :type "SceneComponent Object Reference") (text :type String) (`Tint Color Specified Color` :type "LinearColor Structure") (Justification :type "ETextJustify Enum" :default "Left") (glossaryWord :type "/Game/Blueprints/Enums/GlossaryWords Enum" :default "NewEnumerator6") (OffsetSize :type "Vector2D Structure"))
  (returns (createdPanel :type "/Game/Blueprints/Panels/3DPanel Object Reference"))
  (bind _returnvalue (`|SpawnActorFromClass` (`self.CincinnatiPopUpPrefab`) (`self.K2_GetComponentToWorld` pivot) "Undefined" "OverrideRootScale" null null))
  (bind _as3dpanel (cast `/Game/Blueprints/Panels/3DPanel` _returnvalue))
  (`/Game/Blueprints/Panels/3DPanel.SetupPanel` _as3dpanel text false pivot `Tint Color Specified Color` Justification "Continuar" "" glossaryWord OffsetSize)
  (return _returnvalue))

(fn `ShowGlossaryPopUpPanel`
  (params (pivot :type "SceneComponent Object Reference") (text :type String) (`Tint Color Specified Color` :type "LinearColor Structure") (Justification :type "ETextJustify Enum" :default "Center") (OffsetSize :type "Vector2D Structure") (glossaryWord :type "/Game/Blueprints/Enums/GlossaryWords Enum" :default "NewEnumerator6"))
  (returns (createdPanel :type "/Game/Blueprints/Panels/3DPanel Object Reference"))
  (bind _returnvalue (`|SpawnActorFromClass` (`self.GlossaryPopUpPrefab`) (`self.K2_GetComponentToWorld` pivot) "Undefined" "OverrideRootScale" null null))
  (bind _as3dpanel (cast `/Game/Blueprints/Panels/3DPanel` _returnvalue))
  (`/Game/Blueprints/Panels/3DPanel.SetupPanel` _as3dpanel text false pivot `Tint Color Specified Color` Justification "" "" glossaryWord OffsetSize)
  (return _returnvalue))

(fn `ShowInfoPopUpPanel`
  (params (pivot :type "SceneComponent Object Reference") (text :type String) (b_UseCancelButton :type Boolean) (Justification :type "ETextJustify Enum" :default "Left") (`Tint Color Specified Color` :type "LinearColor Structure" :default (struct :`R` 1.0 :`G` 1.0 :`B` 1.0 :`A` 1.0)) (Button1Text :type String :default "Si") (Button2Text :type String :default "No") (glossaryWord :type "/Game/Blueprints/Enums/GlossaryWords Enum" :default "NewEnumerator6") (OffsetSize :type "Vector2D Structure"))
  (returns (createdPanel :type "/Game/Blueprints/Panels/3DPanel Object Reference"))
  (bind _returnvalue (`|SpawnActorFromClass` (`self.InfoMessagePrefab`) (`self.K2_GetComponentToWorld` pivot) "Undefined" "OverrideRootScale" null null))
  (bind _as3dpanel (cast `/Game/Blueprints/Panels/3DPanel` _returnvalue))
  (`/Game/Blueprints/Panels/3DPanel.SetupPanel` _as3dpanel text b_UseCancelButton pivot `Tint Color Specified Color` Justification Button1Text Button2Text glossaryWord OffsetSize)
  (return _returnvalue))

(fn `ShowSymptomsPanel`
  (params (pivot :type "SceneComponent Object Reference") (text :type String) (`Tint Color Specified Color` :type "LinearColor Structure") (Justification :type "ETextJustify Enum" :default "Left") (glossaryWord :type "/Game/Blueprints/Enums/GlossaryWords Enum" :default "NewEnumerator6") (OffsetSize :type "Vector2D Structure"))
  (returns (createdPanel :type "/Game/Blueprints/Panels/3DPanel Object Reference"))
  (bind _returnvalue (`|SpawnActorFromClass` (`self.symptomsPopUpPrefab`) (`self.K2_GetComponentToWorld` pivot) "Undefined" "OverrideRootScale" null null))
  (bind _as3dpanel (cast `/Game/Blueprints/Panels/3DPanel` _returnvalue))
  (`/Game/Blueprints/Panels/3DPanel.SetupPanel` _as3dpanel text false pivot `Tint Color Specified Color` Justification "Continuar" "" glossaryWord OffsetSize)
  (return _returnvalue))

(fn `ShowTypeOfTestsPanel`
  (params (pivot :type "SceneComponent Object Reference") (text :type String) (`Tint Color Specified Color` :type "LinearColor Structure") (Justification :type "ETextJustify Enum" :default "Left") (glossaryWord :type "/Game/Blueprints/Enums/GlossaryWords Enum" :default "NewEnumerator6") (OffsetSize :type "Vector2D Structure"))
  (returns (createdPanel :type "/Game/Blueprints/Panels/3DPanel Object Reference"))
  (bind _returnvalue (`|SpawnActorFromClass` (`self.TypesOfTestsPopUpPrefab`) (`self.K2_GetComponentToWorld` pivot) "Undefined" "OverrideRootScale" null null))
  (bind _as3dpanel (cast `/Game/Blueprints/Panels/3DPanel` _returnvalue))
  (`/Game/Blueprints/Panels/3DPanel.SetupPanel` _as3dpanel text false pivot `Tint Color Specified Color` Justification "Continuar" "" glossaryWord OffsetSize)
  (return _returnvalue))