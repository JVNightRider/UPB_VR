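; Cinematics manager that plays video on a 3D panel when the player's device nears a target character's head.
; A looping timer measures distance from the skeletal mesh's Head socket to a forward-offset device position, printing it for debug.
; Entering range starts or resumes the VideoWidget; leaving pauses it and hides the panel.
; Media end or FinishScene clears the timer and hides the panel; the too-far warning popup is disconnected.
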(event `self.ReceiveBeginPlay`
  (`parent.ReceiveBeginPlay`))

(event `StartDetectingDistance`
  (params (targetObject :type "SceneComponent Object Reference") (MediaSourceToPlay :type "FileMediaSource Object Reference"))
  (set `self.MediaSource` MediaSourceToPlay)
  (bind _output_get (set `self.targetObject` targetObject))
  (`/Engine/EditorBlueprintResources/StandardMacros.IsValid` _output_get
    (:`Is Valid`
      (set `self.b_isDetectingDistance` true)
      (bind _returnvalue (`KismetSystemLibrary.K2_SetTimer` null "DetectDistanceToTarget" 0.1 true))
      (set `self.TimerDetectingFunction` _returnvalue))))

(event `PlayCinematic`
  (set `self.b_isPlayingVideo` true)
  (set `self.b_isDetectingDistance` false)
  (bind _returnvalue (`GameplayStatics.GetActorOfClass` "/Game/Blueprints/Panels/3DPanelVideo.3DPanelVideo_C"))
  (`Actor.SetActorHiddenInGame` _returnvalue false)
  (bind _asvideo_widget (cast `/Game/Widgets/VideoWidget` (`WidgetComponent.GetUserWidgetObject` (`/Game/Blueprints/Panels/3DPanelVideo.VideoWidget` _returnvalue))))
  (bind _output_get (set `self.VideoWidget` _asvideo_widget))
  (`/Game/Widgets/VideoWidget.PlayVideo` _output_get))

(event `OnMediaFinished`
  (set `self.b_isPlayingVideo` false)
  (set `self.VideoWidget` null)
  (`KismetSystemLibrary.K2_ClearAndInvalidateTimerHandle` (`self.TimerDetectingFunction`))
  (bind _returnvalue (`GameplayStatics.GetActorOfClass` "/Game/Blueprints/Panels/3DPanelVideo.3DPanelVideo_C"))
  (`Actor.SetActorHiddenInGame` _returnvalue true))

(event `PlayerIsTooFar`
  (bind _videowidget (`self.VideoWidget`))
  (set `self.b_isWarningEnable` true)
  (`/Engine/EditorBlueprintResources/StandardMacros.IsValid` _videowidget
    (:`Is Valid`
      (`/Game/Widgets/VideoWidget.PauseVideo` _videowidget)
      (bind _returnvalue (`GameplayStatics.GetActorOfClass` "/Game/Blueprints/Panels/3DPanelVideo.3DPanelVideo_C"))
      (`Actor.SetActorHiddenInGame` _returnvalue true))))

(event `self.FinishScene`
  (bind _videowidget (`self.VideoWidget`))
  (`/Engine/EditorBlueprintResources/StandardMacros.IsValid` _videowidget
    (:`Is Valid`
      (`Widget.RemoveFromParent` _videowidget))
    (:`Is Not Valid`
      _))
  (set `self.b_isPlayingVideo` false)
  (set `self.VideoWidget` null)
  (`KismetSystemLibrary.K2_ClearAndInvalidateTimerHandle` (`self.TimerDetectingFunction`))
  (bind _returnvalue (`GameplayStatics.GetActorOfClass` "/Game/Blueprints/Panels/3DPanelVideo.3DPanelVideo_C"))
  (`Actor.SetActorHiddenInGame` _returnvalue true))

(event `PlayerGetCloser`
  (bind _videowidget (`self.VideoWidget`))
  (set `self.b_isWarningEnable` false)
  (`/Engine/EditorBlueprintResources/StandardMacros.IsValid` _videowidget
    (:`Is Valid`
      (`/Game/Widgets/VideoWidget.ResumeVideo` _videowidget)
      (bind _returnvalue (`GameplayStatics.GetActorOfClass` "/Game/Blueprints/Panels/3DPanelVideo.3DPanelVideo_C"))
      (`Actor.SetActorHiddenInGame` _returnvalue false))))

(fn `DetectDistanceToTarget`
  (bind (_devicerotation _deviceposition) (`HeadMountedDisplayFunctionLibrary.GetOrientationAndPosition`))
  (bind _asskeletal_mesh_component (cast `SkeletalMeshComponent` (`self.targetObject`)))
  (bind _returnvalue (`KismetMathLibrary.Vector_Distance` (`self.GetSocketLocation` _asskeletal_mesh_component "Head") (- _deviceposition (* (`KismetMathLibrary.GetForwardVector` _devicerotation) (1.0 -0.5 1.0)))))
  (`KismetSystemLibrary.PrintString` (`KismetStringLibrary.Conv_DoubleToString` _returnvalue))
  (if (< _returnvalue (`self.triggerVideoDistance`))
    (if (`self.b_isPlayingVideo`)
      (if (`self.b_isWarningEnable`)
        (`self.PlayerGetCloser`))
      (else
        (`self.PlayCinematic`)))
    (elif (`self.b_isPlayingVideo`)
      (if (not (`self.b_isWarningEnable`))
        (`self.PlayerIsTooFar`)))))