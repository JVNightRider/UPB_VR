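; Dialogue manager that serves scene dialogue lines and glossary definitions.
; On BeginPlay it reads the glossary DataTable into word-to-meaning and word-to-internal-glossary maps, skipping one enum value in the latter.
; Dialogue lookup picks one of five DataTables by the SceneFlowManager's current scene index and returns the row's text, glossary word and audio by index.
; Lookup functions query the maps, with that enum value as the internal glossary fallback.
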(event `self.ReceiveBeginPlay`
  (`parent.ReceiveBeginPlay`)
  (`|ExecutionSequence`
    (:`then_0`
      ;[1 1 1] Creates the glosaryMap
      (bind _outrownames (`DataTableFunctionLibrary.GetDataTableRowNames` (`self.GlosaryDataTable`)))
      (for _array_element _outrownames
        (bind _returnvalue (`|GetDataTableRow` (`self.GlosaryDataTable`) _array_element)
          (:`then`
            (bind (_word _meaningtext _internalglossary) (break `/Game/DataTables/GlosaryStructure` _returnvalue))
            (`BlueprintMapLibrary.Map_Add` (`self.GlosaryMap`) _word _meaningtext)
            (if (`|EnumInequality` _internalglossary "NewEnumerator6")
              (`BlueprintMapLibrary.Map_Add` (`self.InternalGlosaryMap`) _word _internalglossary))))))))

(fn `GetDialogActualSceneWithIndex`
  (params (dialogIndex :type Integer))
  (returns (dialogText :type String) (GlossaryWord :type "/Game/Blueprints/Enums/GlossaryWords Enum") (AudioDialog :type "SoundBase Object Reference"))
  (bind _returnvalue (select `int` (`/Game/Blueprints/Managers/SceneFlowManager.actualSceneIndex` (`/Game/Blueprints/Managers/GameManager.SceneFlowManager` (`self.GameManager`))) :`0` (`self.Scene0DialogDataTable`) :`1` (`self.Scene1DialogDataTable`) :`2` (`self.Scene2DialogDataTable`) :`3` (`self.Scene3DialogDataTable`) :`4` (`self.Scene4DialogDataTable`)))
  (bind _outrownames (`DataTableFunctionLibrary.GetDataTableRowNames` _returnvalue))
  (bind _returnvalue_2 (`|GetDataTableRow` _returnvalue (`|GetArrayItem` _outrownames dialogIndex))
    (:`then`
      (bind (_dialog _glossaryword _audiodialog) (break `/Game/DataTables/Dialogs/DialogsStructure` _returnvalue_2))
      (return _dialog _glossaryword _audiodialog))))

(fn `GetGlossaryMeaning`
  (params (Word :type "/Game/Blueprints/Enums/GlossaryWords Enum (by ref)"))
  (returns (TextMeaning :type String))
  (bind (_value _returnvalue) (`BlueprintMapLibrary.Map_Find` (`self.GlosaryMap`) Word))
  (if _returnvalue
    (return _value)))

(fn `GetInternalGlossary`
  (params (Word :type "/Game/Blueprints/Enums/GlossaryWords Enum (by ref)"))
  (returns (Value :type "/Game/Blueprints/Enums/GlossaryWords Enum"))
  (bind (_value _returnvalue) (`BlueprintMapLibrary.Map_Find` (`self.InternalGlosaryMap`) Word))
  (if _returnvalue
    (return _value)
    (else
      (return "NewEnumerator6"))))