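; AnimationsManager is a manager Blueprint that tracks the principal character of the current AR scene object.
; On BeginPlay it binds to the ARManager's scene-object change event through GameManager.
; When a new scene object is detected, it caches that object's PrincipalCharacter and prints a debug string.
; The skeletal-characters RepNotify is empty and no animation is driven here.
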(event `self.ReceiveBeginPlay`
  (`parent.ReceiveBeginPlay`)
  (add `/Game/Blueprints/Managers/ARManager.OnSceneObjectChange` (`/Game/Blueprints/Managers/GameManager.ARManager` (`self.GameManager`)) (delegate `OnNewSceneObjectDetected`)))

(event `OnNewSceneObjectDetected`
  (set `self.Principal Character` (`/Game/Blueprints/SceneObjects/BP_SceneObject.PrincipalCharacter` (`/Game/Blueprints/Managers/ARManager.actualSceneObject` (`/Game/Blueprints/Managers/GameManager.ARManager` (`self.GameManager`)))))
  (`KismetSystemLibrary.PrintString` "pRINCIPAL cHARACTER GETED"))

(fn `OnRep_skeletalCharacters`)