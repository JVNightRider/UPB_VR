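; GameManager Blueprint that starts and finishes scenes in an AR experience.
; Starting delegates the scene index to SceneFlowManager, flags the scene as playing and clears PopUpsManager's toggle answers.
; Finishing resets the flag, notifies MainMenu and destroys every 3DPanel and BP_SceneObject actor.
; It then calls FinishScene on each of its ManagerBase components, so managers clean up through their shared base class, and stops the AR session.
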(event `StartScene`
  (params (SceneIndex :type Integer))
  ;[1 1 1] Start and finish the scene
  (`/Game/Blueprints/Managers/SceneFlowManager.StartScene` (`self.SceneFlowManager`) SceneIndex)
  (set `self.IsPlayingScene` true)
  (`/Game/Blueprints/Managers/PopUpsManager.ClearToggleAnswers` (`self.PopUpsManager`)))

(event `FinishScene`
  ;[1 1 1] Start and finish the scene
  (`|ExecutionSequence`
    (:`then_0`
      (set `self.IsPlayingScene` false)
      (`/Game/Widgets/MainMenu.FinishScene` (`self.MainMenu`)))
    (:`then_1`
      (bind _outactors (`GameplayStatics.GetAllActorsOfClass` "/Game/Blueprints/Panels/3DPanel.3DPanel_C"))
      (for _array_element _outactors
        (`self.K2_DestroyActor` _array_element)))
    (:`then_2`
      (bind _outactors_2 (`GameplayStatics.GetAllActorsOfClass` "/Game/Blueprints/SceneObjects/BP_SceneObject.BP_SceneObject_C"))
      (for _array_element_2 _outactors_2
        (`self.K2_DestroyActor` _array_element_2)))
    (:`then_3`
      (for _array_element_3 (`self.K2_GetComponentsByClass` "/Game/Blueprints/Managers/ManagerBase.ManagerBase_C")
        (`/Game/Blueprints/Managers/ManagerBase.FinishScene` _array_element_3)))
    (:`then_4`
      (`ARBlueprintLibrary.StopARSession`))))

(fn `UserConstructionScript`)